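; Gameplay ability that shoves its avatar when it receives an Event.Push gameplay event.
; It applies a brief additive root motion force along the hit's impact normal from the target data, using the event magnitude as strength and a curve over time.
; GE_PreventMovement is applied to the avatar during the push and removed when the ability ends, which happens when the force finishes.
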(event Ability|EventOnEndAbility
  (params (bWasCancelled :type Boolean))
  (GameplayEffects|RemoveActiveGameplayEffectbySourceEffect (Ability|GetAbilitySystemComponentfromActorInfo) "/Game/PeachCobbler/Blueprints/Ability/GE_PreventMovement.GE_PreventMovement_C" 0 -1))

(event Ability|EventActivateAbilityFromEvent
  (params (EventData :type Gameplay%20Event%20Data%20Structure%20%28by%20ref%29))
  (bind (_eventtag _instigator _target _optionalobject _optionalobject2 _contexthandle _instigatortags _targettags _eventmagnitude _targetdata) (Utilities|Struct|BreakGameplayEventData EventData))
  (|SwitchGameplayTag _eventtag
    (:Event.Push
      (Ability|Tasks|ApplyRootMotionConstantForce "Push" (.ImpactNormal (Collision|BreakHitResult (Ability|TargetData|GetHitResultfromTargetData _targetdata))) _eventmagnitude 0.5 true (Variables|Default|GetPushVelocity) "MaintainLastRootMotionVelocity"
        (:then
          (GameplayEffects|ApplyGameplayEffectToSelf :self (Ability|GetAbilitySystemComponentfromActorInfo) :GameplayEffectClass "/Game/PeachCobbler/Blueprints/Ability/GE_PreventMovement.GE_PreventMovement_C"))
        (:OnFinish
          (Ability|EndAbility))))))