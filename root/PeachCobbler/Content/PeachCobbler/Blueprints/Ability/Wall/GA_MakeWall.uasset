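; Gameplay ability that lets a PeachCobblerCharacter place a wall, using a placer actor during placement.
; Activation from a gameplay event branches on its tag to start placing, place the wall or cancel.
; Starting spawns a placer attached to the character at a rotation-relative offset.
; Placing spawns the wall at that offset from the current transform, only with authority and a valid placer, then destroys the placer, as cancelling does.
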(event Ability|EventActivateAbility)

(event Ability|EventOnEndAbility
  (params (bWasCancelled :type Boolean)))

(event Ability|EventActivateAbilityFromEvent
  (params (EventData :type Gameplay%20Event%20Data%20Structure%20%28by%20ref%29))
  (bind _aspeach_cobbler_character (Utilities|Casting|CastToPeachCobblerCharacter (Ability|GetOwningActorfromActorInfo)))
  (Variables|Default|SetOwningPawn _aspeach_cobbler_character)
  (|SwitchGameplayTag (.EventTag (Utilities|Struct|BreakGameplayEventData EventData))
    (:Event.Wall.StartPlacing
      (bind _returnvalue (Game|SpawnActorfromClass "/Game/PeachCobbler/Blueprints/Ability/Wall/WallPlacer.WallPlacer_C" (CallFunction|GetWallSpawnLocation) "AlwaysSpawn" (Variables|Default|GetOwningPawn) (Variables|Default|GetOwningPawn)))
      (bind _output_get (Variables|Default|SetPlacerWall _returnvalue))
      (Transformation|AttachActorToActor _output_get (Variables|Default|GetOwningPawn) "None" "KeepWorld" "KeepWorld" "KeepWorld" false))
    (:Event.Wall.PlaceWall
      (CallFunction|SpawnWallifAuthority)
      (Actor|DestroyActor (Variables|Default|GetPlacerWall)))
    (:Event.Wall.Cancel
      (Actor|DestroyActor (Variables|Default|GetPlacerWall)))))

(fn OnRepBIsPlacingWall)

(fn SpawnWallifAuthority
  (bind _owningpawn (Variables|Default|GetOwningPawn))
  (if (and (Ability|HasAuthority _owningpawn) (Default|GetIsValid (Variables|Default|GetPlacerWall)))
    (Game|SpawnActorfromClass (Variables|Default|GetWallClass) (CallFunction|GetWallSpawnLocation) "AlwaysSpawn" _owningpawn _owningpawn)))

(fn GetWallSpawnLocation
  (bind _owningpawn (Variables|Default|GetOwningPawn))
  (bind _returnvalue (Transformation|GetActorRotation _owningpawn))
  (return (Math|Transform|MakeTransform (+ (Math|Vector|RotateVector (Variables|Default|GetWallPlacementOffset) _returnvalue) (Transformation|GetActorLocation _owningpawn)) _returnvalue)))