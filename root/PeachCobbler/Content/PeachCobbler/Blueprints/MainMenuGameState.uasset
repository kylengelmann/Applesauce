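; Game state for the main menu that switches the on-screen UI between main, join and lobby menu widgets.
; OpenNewMenu records the requested menu type only with network authority, then on any caller removes the current widget, creates the matching one and adds it to the viewport.
; The event graph and construction script are empty, so switching relies on outside calls to OpenNewMenu.
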(event EventBeginPlay)

(event EventTick
  (params (DeltaSeconds :type Float%20%28single-precision%29)))

(fn ConstructionScript)

(fn OpenNewMenu
  (params (MenuType :type MenuType%20Enum :default "NewEnumerator0"))
  (if (== (Networking|GetLocalRole) 3)
    (Variables|Default|SetCurrentMenuType MenuType))
  (Utilities|IsValid (Variables|Default|GetCurrentMenu)
    (:Is%20Valid
      (Widget|RemovefromParent (Variables|Default|GetCurrentMenu)))
    (:Is%20Not%20Valid
      _))
  (bind _returnvalue (UserInterface|CreateWidget (Utilities|Select :Index MenuType :NewEnumerator0 "/Game/PeachCobbler/Blueprints/MainMenu.MainMenu_C" :NewEnumerator1 "/Game/PeachCobbler/Blueprints/JoinMenu.JoinMenu_C" :NewEnumerator2 "/Game/PeachCobbler/Blueprints/LobbyMenu.LobbyMenu_C")))
  (bind _output_get (Variables|Default|SetCurrentMenu _returnvalue))
  (UserInterface|Viewport|AddtoViewport _output_get 0))