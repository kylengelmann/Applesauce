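; MainMenuManager is a menu-handling Blueprint that shows the main menu on screen at BeginPlay and tracks the active widget in CurrentMenu.
; OpenNewMenu removes the current widget if valid, then creates and displays the main, join or lobby menu chosen by a MenuType selection.
; A separate OpenMainMenu function repeats the BeginPlay logic, adding a main menu without removing the existing one.
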(event EventBeginPlay
  (bind _returnvalue (UserInterface|CreateWidget "/Game/PeachCobbler/Blueprints/MainMenu.MainMenu_C"))
  (bind _output_get (Variables|Default|SetCurrentMenu _returnvalue))
  (UserInterface|Viewport|AddtoViewport _output_get 0))

(fn ConstructionScript)

(fn OpenMainMenu
  (bind _returnvalue (UserInterface|CreateWidget "/Game/PeachCobbler/Blueprints/MainMenu.MainMenu_C"))
  (bind _output_get (Variables|Default|SetCurrentMenu _returnvalue))
  (UserInterface|Viewport|AddtoViewport _output_get 0))

(fn OpenNewMenu
  (params (Menu%20Type :type MenuType%20Enum :default "NewEnumerator0"))
  (Utilities|IsValid (Variables|Default|GetCurrentMenu)
    (:Is%20Valid
      (Widget|RemovefromParent (Variables|Default|GetCurrentMenu)))
    (:Is%20Not%20Valid
      _))
  (bind _returnvalue (UserInterface|CreateWidget (Utilities|Select :Index Menu%20Type :NewEnumerator0 "/Game/PeachCobbler/Blueprints/MainMenu.MainMenu_C" :NewEnumerator1 "/Game/PeachCobbler/Blueprints/JoinMenu.JoinMenu_C" :NewEnumerator2 "/Game/PeachCobbler/Blueprints/LobbyMenu.LobbyMenu_C")))
  (bind _output_get (Variables|Default|SetCurrentMenu _returnvalue))
  (UserInterface|Viewport|AddtoViewport _output_get 0))