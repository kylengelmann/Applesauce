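; PeachCobbler player controller that maps debug-style key presses to push, rock-throw and wall-placement actions on the controlled pawn.
; P calls ServerDoPush, which sends a push gameplay event with a fixed magnitude and a synthetic hit result whose normal opposes the pawn's forward vector.
; Q press and release send gameplay events to start and finish wall placement, while T calls ThrowRock directly on the ThirdPersonCharacter.
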(event Custom|ServerDoPush
  (bind _returnvalue (Pawn|GetControlledPawn))
  (Ability|SendGameplayEventtoActor _returnvalue "(TagName=\"Event.Push\")" (Utilities|Struct|MakeGameplayEventData "" 0 0 0 0 "()" "(GameplayTags=)" "(GameplayTags=)" 1e+01 (Ability|TargetData|AbilityTargetDatafromHitResult (Collision|MakeHitResult false false 0.0 0.0 "0, 0, 0" "0, 0, 0" "0,0,1" (* (Transformation|GetActorForwardVector _returnvalue) -1.0) 0 0)))))

(event EventBeginPlay)

(event EventTick
  (params (DeltaSeconds :type Float%20%28single-precision%29)))

(event Input|KeyboardEvents|P
  (params (Key :type Key%20Structure :default "None"))
  (:Pressed
    (CallFunction|ServerDoPush)))

(event Input|KeyboardEvents|T
  (params (Key :type Key%20Structure :default "None"))
  (:Pressed
    (bind _asthird_person_character (Utilities|Casting|CastToThirdPersonCharacter (Pawn|GetControlledPawn)))
    (Default|ThrowRock _asthird_person_character)))

(event Input|KeyboardEvents|Q
  (params (Key :type Key%20Structure :default "None"))
  (bind _returnvalue (Pawn|GetControlledPawn))
  (:Pressed
    (Ability|SendGameplayEventtoActor _returnvalue "(TagName=\"Event.Wall.StartPlacing\")"))
  (:Released
    (Ability|SendGameplayEventtoActor _returnvalue "(TagName=\"Event.Wall.PlaceWall\")")))

(fn ConstructionScript)